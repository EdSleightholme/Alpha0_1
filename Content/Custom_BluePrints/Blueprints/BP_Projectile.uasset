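; BP_Projectile is a projectile for a tag game that passes the tagger role to the character it strikes.
; Its Sphere's hit and overlap events run duplicate, server-authoritative logic, accepting only untagged characters that can be tagged.
; A successful tag calls RemoveOldTagger on the instigator and SetNewTagger on the target, then destroys all BP_Projectile actors.
; Contact with a non-character destroys only this projectile, while ineligible characters leave it alive.
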(event `self.Sphere.OnComponentHit`
  (params (HitComponent :type "PrimitiveComponent Object Reference") (OtherActor :type "Actor Object Reference") (OtherComp :type "PrimitiveComponent Object Reference") (NormalImpulse :type "Vector Structure") (Hit :type "HitResult Structure (by ref)"))
  (`/Engine/EditorBlueprintResources/ActorMacros.Switch Has Authority`
    (:`Authority`
      ;[1 1 1] See If Can Do Tag Switch
      (bind _asthird_person_character (cast `/Game/Custom_BluePrints/Blueprints/ThirdPersonCharacter` OtherActor)
        (:`then`
          (`/Engine/EditorBlueprintResources/StandardMacros.IsValid` _asthird_person_character
            (:`Is Valid`
              (if (and (not (`/Game/Custom_BluePrints/Blueprints/ThirdPersonCharacter.Tagged` _asthird_person_character)) (`/Game/Custom_BluePrints/Blueprints/ThirdPersonCharacter.CanBeTagged` _asthird_person_character))
                ;[1 1 1] Remove Tagged
                (bind _asthird_person_character_2 (cast `/Game/Custom_BluePrints/Blueprints/ThirdPersonCharacter` (`self.GetInstigator`)))
                (`/Game/Custom_BluePrints/Blueprints/ThirdPersonCharacter.RemoveOldTagger` _asthird_person_character_2)
                ;[1 1 1] Set New Tagger
                (`/Game/Custom_BluePrints/Blueprints/ThirdPersonCharacter.SetNewTagger` _asthird_person_character)
                ;[1 1 1] Destory All Projectiles
                (`KismetSystemLibrary.PrintString` "HITTO")
                (bind _outactors (`GameplayStatics.GetAllActorsOfClass` "BP_Projectile_C"))
                (`self.K2_DestroyActor` _outactors)))
            (:`Is Not Valid`
              (`self.K2_DestroyActor` :!label _label))))
        (:`CastFailed`
          (goto _label))))))

(event `self.Sphere.OnComponentBeginOverlap`
  (params (OverlappedComponent :type "PrimitiveComponent Object Reference") (OtherActor :type "Actor Object Reference") (OtherComp :type "PrimitiveComponent Object Reference") (OtherBodyIndex :type Integer) (bFromSweep :type Boolean) (SweepResult :type "HitResult Structure (by ref)"))
  (`/Engine/EditorBlueprintResources/ActorMacros.Switch Has Authority`
    (:`Authority`
      ;[1 1 1] See If Can Do Tag Switch
      (bind _asthird_person_character (cast `/Game/Custom_BluePrints/Blueprints/ThirdPersonCharacter` OtherActor)
        (:`then`
          (`/Engine/EditorBlueprintResources/StandardMacros.IsValid` _asthird_person_character
            (:`Is Valid`
              (if (and (not (`/Game/Custom_BluePrints/Blueprints/ThirdPersonCharacter.Tagged` _asthird_person_character)) (`/Game/Custom_BluePrints/Blueprints/ThirdPersonCharacter.CanBeTagged` _asthird_person_character))
                ;[1 1 1] Remove Tagged
                (bind _asthird_person_character_2 (cast `/Game/Custom_BluePrints/Blueprints/ThirdPersonCharacter` (`self.GetInstigator`)))
                (`/Game/Custom_BluePrints/Blueprints/ThirdPersonCharacter.RemoveOldTagger` _asthird_person_character_2)
                ;[1 1 1] Set New Tagger
                (`/Game/Custom_BluePrints/Blueprints/ThirdPersonCharacter.SetNewTagger` _asthird_person_character)
                ;[1 1 1] Destory All Projectiles
                (`KismetSystemLibrary.PrintString` "HITTO")
                (bind _outactors (`GameplayStatics.GetAllActorsOfClass` "BP_Projectile_C"))
                (`self.K2_DestroyActor` _outactors)))
            (:`Is Not Valid`
              (`self.K2_DestroyActor` :!label _label_2))))
        (:`CastFailed`
          (goto _label_2))))))

(fn `UserConstructionScript`)